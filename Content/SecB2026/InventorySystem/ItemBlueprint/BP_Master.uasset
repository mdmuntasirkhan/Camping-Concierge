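; BP_Master is a pickup item actor in the inventory system, which the player collects by pressing F while nearby.
; Its collision component enables input on overlap with a BP_Character, stores that character reference, and disables input when an overlap ends.
; Pressing F passes the item's ItemInfo to the character's PickItem and destroys the actor.
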(event `self.Collision.OnComponentBeginOverlap`
  (params (OverlappedComponent :type "PrimitiveComponent Object Reference") (OtherActor :type "Actor Object Reference") (OtherComp :type "PrimitiveComponent Object Reference") (OtherBodyIndex :type Integer) (bFromSweep :type Boolean) (SweepResult :type "HitResult Structure (by ref)"))
  ; Collision Input
  (bind _asbp_character (cast `/Game/SecB2026/Character/BP_Character` OtherActor))
  (set `self.CharacterCast` _asbp_character)
  (`self.EnableInput` (`GameplayStatics.GetPlayerController` 0)))

(event `self.Collision.OnComponentEndOverlap`
  (params (OverlappedComponent :type "PrimitiveComponent Object Reference") (OtherActor :type "Actor Object Reference") (OtherComp :type "PrimitiveComponent Object Reference") (OtherBodyIndex :type Integer))
  ; Collision Input
  (`self.DisableInput` (`GameplayStatics.GetPlayerController` 0)))

(event `Key|F`
  (params (Key :type "Key Structure"))
  ; Collision Input
  (:`Pressed`
    (`/Game/SecB2026/Character/BP_Character.Pick Item` (`self.CharacterCast`) (`self.ItemInfo`))
    (`self.K2_DestroyActor`)))

(fn `UserConstructionScript`)