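; Stove actor with an attached UI widget and a heat effect that responds to a heat level.
; On BeginPlay it casts its widget to WBP_StoveUI and hands it a reference to itself.
; SetHeatIntensity activates FXHeat and drives its User.HeatIntensity Niagara parameter for levels above zero, otherwise it deactivates the effect.
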(event `self.ReceiveBeginPlay`
  ; set stove reference in widget
  (bind _aswbp_stove_ui (cast `/Game/SecB2026/UI/StoveUI/WBP_StoveUI` (`WidgetComponent.GetUserWidgetObject` (`self.Widget`))))
  (set `/Game/SecB2026/UI/StoveUI/WBP_StoveUI.BP_Stove` self _aswbp_stove_ui))

(fn `SetHeatIntensity`
  (params (HeatLevel :type "Float (double-precision)"))
  (bind _fx_heat (`self.FX_Heat`))
  (if (> HeatLevel 0.0)
    (`ActorComponent.Activate` _fx_heat false)
    (`NiagaraComponent.SetVariableFloat` (`self.FX_Heat`) "User.HeatIntensity" (`local.HeatLevel`))
    (else
      (`ActorComponent.Deactivate` _fx_heat))))

(fn `UserConstructionScript`)