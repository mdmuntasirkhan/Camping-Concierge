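; BP_Laptop is an interactable laptop that opens a login screen widget for the player.
; An instruction widget created at BeginPlay appears when the player character overlaps its box and is removed when any actor leaves.
; Interaction passes a DoOnce, shows the login screen with a laptop reference, switches to UI-only input with cursor, and hides the instruction.
; ResetWidget re-arms the DoOnce so the screen can open again.
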(event `self.ReceiveBeginPlay`
  (bind _returnvalue (`|CreateWidget` "/Game/SecB2026/OperatingSystem/Widgets/WBP_Instruction.WBP_Instruction_C"))
  (set `self.InstructionHUD` _returnvalue))

(event `/Game/SecB2026/Blender/Laptop/BPI_Interaction.Interaction`
  (bind _returnvalue (`GameplayStatics.GetPlayerController` 0))
  (`/Engine/EditorBlueprintResources/StandardMacros.DoOnce` false :!label _label
    (:`Completed`
      (bind _returnvalue_2 (`|CreateWidget` "/Game/SecB2026/OperatingSystem/Widgets/WBP_LoginScreen.WBP_LoginScreen_C"))
      (`UserWidget.AddToPlayerScreen` _returnvalue_2 0)
      (set `/Game/SecB2026/OperatingSystem/Widgets/WBP_LoginScreen.Laptop` self _returnvalue_2)
      (`WidgetBlueprintLibrary.SetInputMode_UIOnlyEx` _returnvalue _returnvalue_2)
      (set `PlayerController.bShowMouseCursor` true _returnvalue)
      (`Widget.RemoveFromParent` (`self.InstructionHUD`)))))

(event `ResetWidget`
  (goto _label :!via `Reset`))

(event `self.Box.OnComponentBeginOverlap`
  (params (OverlappedComponent :type "PrimitiveComponent Object Reference") (OtherActor :type "Actor Object Reference") (OtherComp :type "PrimitiveComponent Object Reference") (OtherBodyIndex :type Integer) (bFromSweep :type Boolean) (SweepResult :type "HitResult Structure (by ref)"))
  ; Show the interaction button
  (if (== OtherActor (`GameplayStatics.GetPlayerCharacter` 0))
    (`UserWidget.AddToViewport` (`self.InstructionHUD`) 0)))

(event `self.Box.OnComponentEndOverlap`
  (params (OverlappedComponent :type "PrimitiveComponent Object Reference") (OtherActor :type "Actor Object Reference") (OtherComp :type "PrimitiveComponent Object Reference") (OtherBodyIndex :type Integer))
  ; Hide the interaction button
  (if true
    (`Widget.RemoveFromParent` (`self.InstructionHUD`))))

(fn `UserConstructionScript`)