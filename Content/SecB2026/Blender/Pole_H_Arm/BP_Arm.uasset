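; BP_Arm is a barrier gate arm that toggles between open and closed when OpenArmGate is called.
; The event checks IsArmOpen and plays one of two timelines from the start, lerping the PoleHArm pitch between 0 and 90 degrees.
; IsArmOpen flips on timeline update rather than on finish, so a call mid-swing restarts in the opposite direction from that swing's end angle.
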(event `OpenArmGate`
  (if (`self.IsArmOpen?`)
    (bind (_direction _armfloat) (`Timeline|Timeline_0` :!via `PlayFromStart`)
      (:`Update`
        (`SceneComponent.K2_SetRelativeRotation` (`self.Pole_H_arm`) (`KismetMathLibrary.MakeRotator` 0.0 (`KismetMathLibrary.Lerp` 90.0 0.0 _armfloat)) false false)
        (set `self.IsArmOpen?` false)))
    (else
      (bind (_direction_2 _armfloat_2) (`Timeline|Timeline` :!via `PlayFromStart`)
        (:`Update`
          (`SceneComponent.K2_SetRelativeRotation` (`self.Pole_H_arm`) (`KismetMathLibrary.MakeRotator` 0.0 (`KismetMathLibrary.Lerp` 0.0 90.0 _armfloat_2)) false false)
          (set `self.IsArmOpen?` true))))))

(fn `UserConstructionScript`)