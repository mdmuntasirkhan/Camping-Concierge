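; Van actor that lets a character inside it switch between the character camera and the van's kitchen camera.
; Interaction checks BP_Character overlaps in InteriorCollisionBox and either returns a VanMode character to its camera or sets the van as VanViewTarget and switches to the kitchen view.
; Two functions apply relative yaw and inverted pitch to KitchenCamera.
; BeginPlay creates an instruction widget without adding it to the viewport.
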(event `self.ReceiveBeginPlay`
  (`|CreateWidget` "/Game/SecB2026/OperatingSystem/Widgets/WBP_Instruction.WBP_Instruction_C"))

(event `/Game/SecB2026/Blender/Laptop/BPI_Interaction.Interaction`
  (for _array_element (`PrimitiveComponent.GetOverlappingActors` (`self.InteriorCollisionBox`) "/Game/SecB2026/Character/BP_Character.BP_Character_C")
    (bind _asbp_character (cast `/Game/SecB2026/Character/BP_Character` _array_element))
    (if (`/Game/SecB2026/Character/BP_Character.VanMode` _asbp_character)
      (`/Game/SecB2026/Character/BP_Character.SwitchBackToCharacterCamera` _asbp_character)
      (else
        (set `/Game/SecB2026/Character/BP_Character.VanViewTarget` self _asbp_character)
        (`/Game/SecB2026/Character/BP_Character.SwitchToKitchenCamera` _asbp_character)
        (`KismetSystemLibrary.PrintString` "work")
        (break)))))

(fn `RotateCameraHorizentally`
  (params (RotateValue :type "Float (double-precision)"))
  (`SceneComponent.K2_AddRelativeRotation` (`self.KitchenCamera`) (`KismetMathLibrary.MakeRotator` 0.0 0.0 RotateValue) false false))

(fn `RotateCameraVerticaly`
  (params (RotateValue :type "Float (double-precision)"))
  (`SceneComponent.K2_AddRelativeRotation` (`self.KitchenCamera`) (`KismetMathLibrary.MakeRotator` 0.0 (* RotateValue -1.0)) false false))

(fn `UserConstructionScript`)