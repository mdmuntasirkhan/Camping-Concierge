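; BP_NPC is an NPC Blueprint that shows its dialog lines one at a time on screen.
; Each Talk event increments TalkIntex, then writes that Dialog array entry into a WBP_Dialog widget, created and added to the viewport if the stored reference is invalid.
; Once the index exceeds the array length, the widget is removed from its parent, and the index is not reset.
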(event `/Game/SecB2026/CharacterNPC/Dialog/BPI_Dialog.Talk`
  (`/Engine/EditorBlueprintResources/StandardMacros.IncrementInt` (`self.Talk_Intex`)
    (:`  `
      (if (<= (`self.Talk_Intex`) (`KismetArrayLibrary.Array_Length` (`self.Dialog`)))
        (`self.UI_Dialog`
          (:`then`
            _)
          (:`else`
            (bind _returnvalue (`|CreateWidget` "/Game/SecB2026/UI/NPC_Dialog/WBP_Dialog.WBP_Dialog_C" (`GameplayStatics.GetPlayerController` 0)))
            (bind _output_get (set `self.UI_Dialog` _returnvalue))
            (`UserWidget.AddToViewport` _output_get 0)))
        (`TextBlock.SetText` (`/Game/SecB2026/UI/NPC_Dialog/WBP_Dialog.Dialog_Text` (`self.UI_Dialog`)) (`KismetTextLibrary.Conv_StringToText` (`|GetArrayItem` (`self.Dialog`) (`self.Talk_Intex`))))
        (else
          (`Widget.RemoveFromParent` (`self.UI_Dialog`)))))))

(fn `UserConstructionScript`)