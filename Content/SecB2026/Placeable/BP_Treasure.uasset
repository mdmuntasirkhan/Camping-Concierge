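; BP_Treasure is a placeable treasure chest with an animated lid and a one-time pickup.
; ChestOpen toggles the lid, using one of two timelines to lerp the mesh pitch open or closed.
; CharacterOverlap updates the passed character's treasure count once, then swaps the glow and aura audio for collection VFX and a pickup sound.
; Later overlaps only print an already-collected message.
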(event `ChestOpen`
  ; Door Open
  (if (`self.IsChestOpen`)
    (bind (_direction _doorfloat) (`Timeline|Timeline` :!via `PlayFromStart`)
      (:`Update`
        (`SceneComponent.K2_SetRelativeRotation` (`self.StaticMesh1`) (`KismetMathLibrary.MakeRotator` 0.0 (`KismetMathLibrary.Lerp` -90.0 0.0 _doorfloat)) false false)
        (set `self.IsChestOpen` false)))
    (else
      (bind (_direction_2 _doorfloat_2) (`Timeline|Timeline_0` :!via `PlayFromStart`)
        (:`Update`
          (`SceneComponent.K2_SetRelativeRotation` (`self.StaticMesh1`) (`KismetMathLibrary.MakeRotator` 0.0 (`KismetMathLibrary.Lerp` 0.0 -90.0 _doorfloat_2)) false false)
          (set `self.IsChestOpen` true))))))

(fn `CharacterOverlap`
  (params (CharacterRef :type "/Game/SecB2026/Character/BP_Character Object Reference"))
  ; Update Treasure
  (if (`self.bCollected`)
    (`KismetSystemLibrary.PrintString` "Treasure Already Collected" true true (struct :`R` 1.0 :`G` 0.001687 :`B` 0.479632 :`A` 1.0))
    (else
      (`/Game/SecB2026/Character/BP_Character.UpdateTreasureNumber` CharacterRef)
      (set `self.bCollected` true)
      (`self.UpdateVFX`)
      (`self.UpdateSFX`))))

(fn `UpdateSFX`
  ; Update SFX and Spawning a new sounnd
  (`AudioComponent.Stop` (`self.TreasureAuraAudio`))
  (`GameplayStatics.SpawnSoundAtLocation` "/Game/SecB2026/Audio/SFX/A_GoldPickup_Cue.A_GoldPickup_Cue" (`self.K2_GetActorLocation`) (struct) 1.0 1.0 0.0 null null))

(fn `UpdateVFX`
  (bind _glowingeffect (`self.GlowingEffect`))
  ; Deactivate VFX
  (`ActorComponent.Deactivate` _glowingeffect)
  ; Spawn new VFX
  (`NiagaraFunctionLibrary.SpawnSystemAtLocation` "/Game/SecB2026/Effects/FXS_TreasureCollected.FXS_TreasureCollected" (`SceneComponent.K2_GetComponentLocation` _glowingeffect)))

(fn `UserConstructionScript`
  (`parent.UserConstructionScript`))